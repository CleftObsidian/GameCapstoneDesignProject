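; Placard actor that sways the wind acting on its VerletClothMesh cloth component.
; Each Tick steps an angle one degree, reversing direction past 65 degrees either side of zero, and converts it with cosine and sine into a horizontal WindDirection vector.
; The sweep ignores delta time, so its speed depends on frame rate.
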(event EventBeginPlay)

(event Collision|EventActorBeginOverlap
  (params (OtherActor :type Actor%20Object%20Reference)))

(event EventTick
  (params (DeltaSeconds :type Float%20%28single-precision%29))
  (if (> (Variables|Default|Getangle) 65.0)
    (Variables|Default|Setdir -1)
    (elif (< (Variables|Default|Getangle) -65.0)
      (Variables|Default|Setdir 1)))
  (Variables|Default|Setangle (+ (Variables|Default|Getangle) (* (Variables|Default|Getdir) 1.0)))
  (Variables|/Script/VerletClothMesh.VerletClothMeshComponent|SetWindDirection (Variables|Default|GetVerletClothMesh) (Math|Vector|MakeVector (Math|Trig|Cos(Degrees) (Variables|Default|Getangle)) (Math|Trig|Sin(Degrees) (Variables|Default|Getangle)) 0.0)))

(fn ConstructionScript)